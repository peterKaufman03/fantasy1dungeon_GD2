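; BP_CellDoor is a cell door that opens only once every collectable has been gathered.
; When the first-person character overlaps its Collision volume, it reads CollectableLeft from the game mode.
; At zero it snaps the door mesh to an open rotation and plays the Grave_Mistake 2D sound event once; otherwise it prints a "Missing Keys" message.
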(event `self.Collision.OnComponentBeginOverlap`
  (params (OverlappedComponent :type "PrimitiveComponent Object Reference") (OtherActor :type "Actor Object Reference") (OtherComp :type "PrimitiveComponent Object Reference") (OtherBodyIndex :type Integer) (bFromSweep :type Boolean) (SweepResult :type "HitResult Structure (by ref)"))
  (cast `/Game/FirstPerson/Blueprints/BP_FirstPersonCharacter` OtherActor)
  (bind _asbp_first_person_game_mode (cast `/Game/FirstPerson/Blueprints/BP_FirstPersonGameMode` (`GameplayStatics.GetGameMode`)))
  (if (== (`/Game/FirstPerson/Blueprints/BP_FirstPersonGameMode.CollectableLeft` _asbp_first_person_game_mode) 0)
    (`SceneComponent.K2_SetRelativeRotation` (`self.SM_Bld_Cell_Door_01_Door_01`) (struct :`Yaw` -110.0) false false)
    (`/Engine/EditorBlueprintResources/StandardMacros.DoOnce` false
      (:`Completed`
        (`FMODBlueprintStatics.PlayEvent2D` "/Game/FMOD/Events/Dialogue/Beholder_Dialogue/Grave_Mistake.Grave_Mistake")))
    (else
      (`KismetSystemLibrary.PrintString` "Missing Keys" true true (struct :`R` 0.222647 :`G` 0.08849 :`B` 1.0 :`A` 1.0)))))

(fn `UserConstructionScript`)