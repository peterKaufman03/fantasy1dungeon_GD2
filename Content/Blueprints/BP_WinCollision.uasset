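; BP_WinCollision is a win trigger that starts the victory and credits sequence when BP_FirstPersonCharacter overlaps its Collision component.
; On overlap it creates a win widget, adds it to the viewport and plays its Fade animation.
; After a delay it adds W_Credits on top and staggers the text and per-name fade-in animations with short delays.
; The chain ends on a final delay with nothing after it, and nothing guards against repeat overlaps.
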(event `self.Collision.OnComponentBeginOverlap`
  (params (OverlappedComponent :type "PrimitiveComponent Object Reference") (OtherActor :type "Actor Object Reference") (OtherComp :type "PrimitiveComponent Object Reference") (OtherBodyIndex :type Integer) (bFromSweep :type Boolean) (SweepResult :type "HitResult Structure (by ref)"))
  (cast `/Game/FirstPerson/Blueprints/BP_FirstPersonCharacter` OtherActor)
  (bind _returnvalue (`|CreateWidget` "/Game/WidgetsUI/W_Win.W_Win_C"))
  (`UserWidget.AddToViewport` _returnvalue 0)
  (`UserWidget.PlayAnimation` _returnvalue (`/Game/WidgetsUI/W_Win.Fade` _returnvalue) 0.0 1 "Forward" 1.0 false)
  (`KismetSystemLibrary.Delay` 5.0)
  (bind _returnvalue_2 (`|CreateWidget` "/Game/WidgetsUI/W_Credits.W_Credits_C"))
  (`UserWidget.AddToViewport` _returnvalue_2 0)
  (`UserWidget.PlayAnimation` _returnvalue_2 (`/Game/WidgetsUI/W_Credits.TextFadeIn` _returnvalue_2) 0.0 1 "Forward" 1.0 false)
  (`KismetSystemLibrary.Delay` 0.15)
  (`UserWidget.PlayAnimation` _returnvalue_2 (`/Game/WidgetsUI/W_Credits.PeterFadeIn` _returnvalue_2) 0.0 1 "Forward" 1.0 false)
  (`KismetSystemLibrary.Delay` 0.15)
  (`UserWidget.PlayAnimation` _returnvalue_2 (`/Game/WidgetsUI/W_Credits.YoungFadeIn` _returnvalue_2) 0.0 1 "Forward" 1.0 false)
  (`KismetSystemLibrary.Delay` 0.15)
  (`UserWidget.PlayAnimation` _returnvalue_2 (`/Game/WidgetsUI/W_Credits.BenFadeIn` _returnvalue_2) 0.0 1 "Forward" 1.0 false)
  (`KismetSystemLibrary.Delay` 0.15)
  (`UserWidget.PlayAnimation` _returnvalue_2 (`/Game/WidgetsUI/W_Credits.NateFadeIn` _returnvalue_2) 0.0 1 "Forward" 1.0 false)
  (`KismetSystemLibrary.Delay` 5.0))

(fn `UserConstructionScript`)