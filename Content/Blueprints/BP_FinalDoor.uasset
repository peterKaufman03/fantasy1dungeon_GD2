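; BP_FinalDoor is a door actor that opens only after the player has gathered every collectable.
; When the first-person character overlaps its Collision, it reads CollectableLeft from BP_FirstPersonGameMode.
; At zero, a Timeline lerps the Door's relative location downward to open it; otherwise it prints a "Missing Keys" message.
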(event `self.Collision.OnComponentBeginOverlap`
  (params (OverlappedComponent :type "PrimitiveComponent Object Reference") (OtherActor :type "Actor Object Reference") (OtherComp :type "PrimitiveComponent Object Reference") (OtherBodyIndex :type Integer) (bFromSweep :type Boolean) (SweepResult :type "HitResult Structure (by ref)"))
  (cast `/Game/FirstPerson/Blueprints/BP_FirstPersonCharacter` OtherActor)
  (bind _asbp_first_person_game_mode (cast `/Game/FirstPerson/Blueprints/BP_FirstPersonGameMode` (`GameplayStatics.GetGameMode`)))
  (if (== (`/Game/FirstPerson/Blueprints/BP_FirstPersonGameMode.CollectableLeft` _asbp_first_person_game_mode) 0)
    (bind (_direction _newtrack_0) (`Timeline|Timeline`)
      (:`Update`
        (`SceneComponent.K2_SetRelativeLocation` (`self.Door`) (`KismetMathLibrary.VLerp` (0.0 0.0 150.0) (0.0 0.0 -130.0) _newtrack_0) false false)))
    (else
      (`KismetSystemLibrary.PrintString` "Missing Keys" true true (struct :`R` 0.222647 :`G` 0.08849 :`B` 1.0 :`A` 1.0)))))

(fn `UserConstructionScript`)