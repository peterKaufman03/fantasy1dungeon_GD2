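; Spike trap that moves its Box vertically and detects when the first-person character touches it.
; On BeginPlay, the RiseAndFall timeline drives the Box's relative Z, while a self-looping Delay replays the first entry in Sounds every few seconds, independently of the timeline.
; Overlap with BP_FirstPersonCharacter only prints a death message, with no damage or kill logic.
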(event `self.ReceiveBeginPlay`
  (`|ExecutionSequence`
    (:`then_0`
      (bind (_direction _newtrack_0) (`Timeline|Rise and Fall`)
        (:`Update`
          (`SceneComponent.K2_SetRelativeLocation` (`self.Box`) (`KismetMathLibrary.MakeVector` 0.0 0.0 (- (* _newtrack_0 70.0) 110.0)) false false))))
    (:`then_1`
      (`KismetSystemLibrary.Delay` 3.0 :!label _label)
      (`self.Sound` 0)
      (goto _label))))

(event `self.Box.OnComponentBeginOverlap`
  (params (OverlappedComponent :type "PrimitiveComponent Object Reference") (OtherActor :type "Actor Object Reference") (OtherComp :type "PrimitiveComponent Object Reference") (OtherBodyIndex :type Integer) (bFromSweep :type Boolean) (SweepResult :type "HitResult Structure (by ref)"))
  (cast `/Game/FirstPerson/Blueprints/BP_FirstPersonCharacter` OtherActor)
  (`KismetSystemLibrary.PrintString` "And Dead"))

(event `Sound`
  (params (`Dimension 1` :type Integer))
  (`AudioComponent.SetSound` (`self.Audio`) (`|GetArrayItem` (`self.Sounds`) `Dimension 1`))
  (`AudioComponent.Play` (`self.Audio`) 0.0))

(fn `UserConstructionScript`)